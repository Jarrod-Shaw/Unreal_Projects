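; Player controller that flies the possessed BP_AircraftBASE, cached on BeginPlay.
; Pitch, yaw and roll axis inputs apply local rotation to the aircraft directly.
; Throttle inputs run self-repeating Delay loops that step a clamped Throttle while held, with a shorter delay for throttling down, and the afterburner input toggles the aircraft's flag while held.
; Weapon, camera, radial menu and direction functions are empty stubs; AngleOfAttack computes the angle between two vectors.
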(event `self.ReceiveBeginPlay`
  (bind _returnvalue (`self.K2_GetPawn`))
  (`/Engine/EditorBlueprintResources/StandardMacros.IsValid` _returnvalue
    (:`Is Valid`
      (bind _asbp_aircraft_base (cast `/Game/BluePrints/BP_AircraftBASE` _returnvalue)))))

(event `self.ReceiveTick`
  (params (DeltaSeconds :type "Float (single-precision)"))
  ;[1 1 1] Event Tick
)

(event `InputAxis|Pitch`
  (params (AxisValue :type "Float (single-precision)"))
  ;[1 1 1] Pitch
  (`self.K2_AddActorLocalRotation` (stale `self.ReceiveBeginPlay` _asbp_aircraft_base) (`KismetMathLibrary.MakeRotator` 0.0 (+ AxisValue (* (`self.GetInputAxisValue`) (`GameplayStatics.GetWorldDeltaSeconds`)))) false false))

(event `ThrottleUp`
  ;[1 1 1] Throttle Up
  (`KismetSystemLibrary.Delay` (`GameplayStatics.GetWorldDeltaSeconds`) :!label _label)
  (set `/Game/BluePrints/BP_AircraftBASE.Throttle` (`KismetMathLibrary.FClamp` (+ (`/Game/BluePrints/BP_AircraftBASE.Throttle` (stale `self.ReceiveBeginPlay` _asbp_aircraft_base)) (`self.ThrottleRate`)) 0.0 100.0) (stale `self.ReceiveBeginPlay` _asbp_aircraft_base))
  (if (`self.Is_ThrottlingUp`)
    (goto _label)))

(event `InputAction|ThrottleUp`
  (params (Key :type "Key Structure"))
  ;[1 1 1] Throttle Up
  (:`Pressed`
    (set `self.Is_ThrottlingUp` true)
    (`self.ThrottleUp` :!label _label_2))
  (:`Released`
    (set `self.Is_ThrottlingUp` false)
    (goto _label_2)))

(event `InputAxis|Yaw`
  (params (AxisValue :type "Float (single-precision)"))
  ;[1 1 1] Yaw
  (`self.K2_AddActorLocalRotation` (stale `self.ReceiveBeginPlay` _asbp_aircraft_base) (`KismetMathLibrary.MakeRotator` 0.0 0.0 (+ AxisValue (* (`self.GetInputAxisValue`) (`GameplayStatics.GetWorldDeltaSeconds`)))) false false))

(event `ThrottleDwn`
  ;[1 1 1] Throttle Down
  (`KismetSystemLibrary.Delay` (* (`GameplayStatics.GetWorldDeltaSeconds`) 0.1) :!label _label_3)
  (set `/Game/BluePrints/BP_AircraftBASE.Throttle` (`KismetMathLibrary.FClamp` (- (`/Game/BluePrints/BP_AircraftBASE.Throttle` (stale `self.ReceiveBeginPlay` _asbp_aircraft_base)) (`self.ThrottleRate`)) 0.0 100.0) (stale `self.ReceiveBeginPlay` _asbp_aircraft_base))
  (if (`self.Is_ThrottlingDwn`)
    (goto _label_3)))

(event `InputAction|ThrottleDown`
  (params (Key :type "Key Structure"))
  ;[1 1 1] Throttle Down
  (:`Pressed`
    (set `self.Is_ThrottlingDwn` true)
    (`self.ThrottleDwn` :!label _label_4))
  (:`Released`
    (set `self.Is_ThrottlingDwn` false)
    (goto _label_4)))

(event `InputAxis|Roll`
  (params (AxisValue :type "Float (single-precision)"))
  ;[1 1 1] Roll
  (`self.K2_AddActorLocalRotation` (stale `self.ReceiveBeginPlay` _asbp_aircraft_base) (`KismetMathLibrary.MakeRotator` (+ AxisValue (* (`self.GetInputAxisValue`) (`GameplayStatics.GetWorldDeltaSeconds`)))) false false))

(event `Speed`)

(event `InputAction|AfterBurner`
  (params (Key :type "Key Structure"))
  ;[1 1 1] Afterburner
  (:`Pressed`
    (set `/Game/BluePrints/BP_AircraftBASE.Is_AfterBurnerOn` true (stale `self.ReceiveBeginPlay` _asbp_aircraft_base)))
  (:`Released`
    (set `/Game/BluePrints/BP_AircraftBASE.Is_AfterBurnerOn` false (stale `self.ReceiveBeginPlay` _asbp_aircraft_base))))

(fn `AngleOfAttack`
  (params (VectorA :type "Vector Structure") (VectorB :type "Vector Structure"))
  (returns (`Angle (Rad)` :type "Float (double-precision)"))
  (bind _returnvalue (`KismetMathLibrary.Acos` (`KismetMathLibrary.Dot_VectorVector` (`KismetMathLibrary.Normal` VectorA) (`KismetMathLibrary.Normal` VectorB))))
  (if true
    (return _returnvalue)
    (else
      (return (* _returnvalue -1.0)))))

(fn `ChangeCamera`)

(fn `FireGun`)

(fn `FireMissile`)

(fn `GetDirection`)

(fn `RadialMenu`)

(fn `UserConstructionScript`)