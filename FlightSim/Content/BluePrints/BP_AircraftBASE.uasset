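; Base aircraft Blueprint that prototypes a simple forward-flight model from engine count, thrust, weight and drag.
; BeginPlay sums the weight and sets starting throttle; Tick recalculates thrust (afterburner or throttled dry), speed and acceleration, printing each for debugging.
; Acceleration comes from thrust over weight, and speed integrates it minus drag.
; It is unfinished: the actor offset is zero, drag and lift events are empty, and altitude only resets to zero.
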(event `self.ReceiveBeginPlay`
  (set `self.Throttle` 85.0)
  (set `self.CurrentWeight` (+ (`self.EmptyWeight`) (`self.FuelWeight`) (`self.ArmamentsWeight`)))
  (set `self.Altitude` 0.0))

(event `self.ReceiveTick`
  (params (DeltaSeconds :type "Float (single-precision)"))
  (`self.Calc_ForwardThrust`)
  (`self.Calc_Speed`)
  (`self.Calc_Acceleration`)
  (`self.K2_AddActorLocalOffset` (`KismetMathLibrary.MakeVector` 0.0)))

(event `Calc_ForwardThrust`
  (bind _returnvalue (`GameplayStatics.GetWorldDeltaSeconds`))
  ;[1 1 1] Forward Thrust -> Afterburner
  (if (`self.Is_AfterBurnerOn`)
    (bind _output_get (set `self.ForwardThrust` (* (* (`self.NumberOfEngines`) (`self.AfterBurnerThrust`)) 100.0)))
    (`KismetSystemLibrary.PrintString` (`KismetStringLibrary.Conv_DoubleToString` _output_get) true true (struct :`R` 1.0 :`A` 1.0) _returnvalue)
    (else
      (bind _output_get_2 (set `self.ForwardThrust` (* (* (`self.NumberOfEngines`) (`self.DryThrust`)) (`self.Throttle`))))
      (`KismetSystemLibrary.PrintString` (`KismetStringLibrary.Conv_DoubleToString` _output_get_2) true true (struct :`B` 1.0 :`A` 1.0) _returnvalue))))

(event `Calc_Acceleration`
  (bind _returnvalue (`GameplayStatics.GetWorldDeltaSeconds`))
  ;[1 1 1] Acceleration = force / mass vs Resistance
  (bind _output_get (set `self.Acceleration` (* (/ (`self.ForwardThrust`) (`self.CurrentWeight`)) _returnvalue)))
  (`KismetSystemLibrary.PrintString` (`KismetStringLibrary.Conv_DoubleToString` _output_get) true true (struct :`G` 0.66 :`B` 1.0 :`A` 1.0) _returnvalue))

(event `Calc_Speed`
  (bind _returnvalue (`GameplayStatics.GetWorldDeltaSeconds`))
  ;[1 1 1] Speed = (Accelleration +/- speed) - Drag
  (bind _output_get (set `self.ForwardSpeed` (+ (- (* (`self.Acceleration`) _returnvalue) (* _returnvalue (`self.Drag`))) (`self.ForwardSpeed`))))
  (`KismetSystemLibrary.PrintString` (`KismetStringLibrary.Conv_DoubleToString` _output_get) true true (struct :`R` 0.197917 :`G` 0.197917 :`B` 0.197917 :`A` 1.0) _returnvalue))

(event `Calc_Altitude`
  ;[1 1 1] Altitude
  (set `self.Altitude` 0.0))

(event `Calc_Drag`
  ;[1 1 1] WR = Air Density * DragCoefficient
)

(event `Lift_Overcome_Gravity`)

(fn `UserConstructionScript`)